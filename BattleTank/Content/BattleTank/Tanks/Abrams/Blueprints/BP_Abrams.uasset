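; Player-drivable Abrams tank Blueprint that wires its components and input to the tank's movement, camera and firing.
; BeginPlay passes barrel and turret references to the tank's setters and initialises TankMovement with both tracks.
; Input drives either per-track throttles directly or forward and turn intents through TankMovement.
; Aim axes rotate an azimuth gimbal for yaw and the spring arm for pitch, scaled by delta time, and Fire calls the fire function.
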(event `self.ReceiveBeginPlay`
  (`self.SetBarrelReference` (`self.TankBarrel`))
  (`self.SetTurretReference` (`self.TankTurret`))
  (`TankMovementComponent.Initalise` (`self.TankMovement`) (`self.LeftTracks`) (`self.RightTracks`)))

(event `InputAxis|LeftTrackThrottle`
  (params (AxisValue :type "Float (single-precision)"))
  ;[1 1 1] Tank Axis Throttle Controls
  (`TankTracks.SetThrottle` (`self.LeftTracks`) AxisValue))

(event `InputAxis|AimAzimuth`
  (params (AxisValue :type "Float (single-precision)"))
  ;[1 1 1] Camera Input Binding
  (`SceneComponent.K2_AddLocalRotation` (`self.Azimuth Gimbal`) (`KismetMathLibrary.MakeRotator` 0.0 0.0 (* AxisValue (`GameplayStatics.GetWorldDeltaSeconds`) 100.0)) false false))

(event `InputAxis|RightTrackThrottle`
  (params (AxisValue :type "Float (single-precision)"))
  ;[1 1 1] Tank Axis Throttle Controls
  (`TankTracks.SetThrottle` (`self.RightTracks`) AxisValue))

(event `InputAxis|AimElevation`
  (params (AxisValue :type "Float (single-precision)"))
  ;[1 1 1] Camera Input Binding
  (`SceneComponent.K2_AddLocalRotation` (`self.SpringArm`) (`KismetMathLibrary.MakeRotator` 0.0 (* AxisValue (`GameplayStatics.GetWorldDeltaSeconds`) 100.0)) false false))

(event `InputAxis|ForwardMovement`
  (params (AxisValue :type "Float (single-precision)"))
  ;[1 1 1] Tank Axis Throttle Controls
  (`TankMovementComponent.IntendMoveForward` (`self.TankMovement`) AxisValue))

(event `InputAxis|TurnRigh`
  (params (AxisValue :type "Float (single-precision)"))
  ;[1 1 1] Tank Axis Throttle Controls
  (`TankMovementComponent.IntendMoveRight` (`self.TankMovement`) AxisValue))

(event `InputAction|Fire`
  (params (Key :type "Key Structure" :default "AnyKey"))
  ;[1 1 1] Firing Input Binding
  (:`Pressed`
    (`self.Fire`)))

(fn `UserConstructionScript`)